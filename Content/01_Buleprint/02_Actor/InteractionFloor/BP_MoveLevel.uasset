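; BP_MoveLevel is a level-transition trigger actor that sends the game to another level when the player's character steps into it.
; When a BP_Base_character begins overlapping its Box, it starts its RotatingMovement spinning and immediately opens the level referenced by the Level variable.
; When that character leaves the Box, the rotation rate resets to zero.
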(event OnComponentBeginOverlap(Box)
  (params (OverlappedComponent :type Primitive%20Component%20Object%20Reference) (OtherActor :type Actor%20Object%20Reference) (OtherComp :type Primitive%20Component%20Object%20Reference) (OtherBodyIndex :type Integer) (bFromSweep :type Boolean) (SweepResult :type Hit%20Result%20Structure%20%28by%20ref%29))
  (bind _asbp_base_character (Utilities|Casting|CastToBP_Base_character OtherActor))
  (Utilities|IsValid _asbp_base_character
    (:Is%20Valid
      (Variables|/Script/Engine.RotatingMovementComponent|SetRotationRate (Variables|Default|GetRotatingMovement) "0.000000,180.000000,0.000000")
      (Game|OpenLevel(byObjectReference) (Variables|Default|GetLevel)))))

(event OnComponentEndOverlap(Box)
  (params (OverlappedComponent :type Primitive%20Component%20Object%20Reference) (OtherActor :type Actor%20Object%20Reference) (OtherComp :type Primitive%20Component%20Object%20Reference) (OtherBodyIndex :type Integer))
  (bind _asbp_base_character (Utilities|Casting|CastToBP_Base_character OtherActor))
  (Utilities|IsValid _asbp_base_character
    (:Is%20Valid
      (Variables|/Script/Engine.RotatingMovementComponent|SetRotationRate (Variables|Default|GetRotatingMovement) "0, 0, 0"))))

(event EventBeginPlay)

(event Collision|EventActorBeginOverlap
  (params (OtherActor :type Actor%20Object%20Reference)))

(event EventTick
  (params (DeltaSeconds :type Float%20%28single-precision%29)))

(fn ConstructionScript)