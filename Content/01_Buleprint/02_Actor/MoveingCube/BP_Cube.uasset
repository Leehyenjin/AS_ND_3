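; BP_Cube is a moving cube actor that shuttles back and forth along its Dir vector, commented as rising and descending.
; Each Tick accumulates AccTime and offsets the location by normalized Dir times Speed and delta time, forward or reversed depending on the Go flag.
; When AccTime exceeds five seconds, Go flips and the timer resets.
; Movement uses no sweep, so collisions do not block it.
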(event EventBeginPlay)

(event Collision|EventActorBeginOverlap
  (params (OtherActor :type Actor%20Object%20Reference)))

(event EventTick
  (params (DeltaSeconds :type Float%20%28single-precision%29))
  (Utilities|FlowControl|Sequence
    (:then_0
      ;[1 1 1] AccTime값 증가
      (Variables|Default|SetAccTime (+ (Variables|Default|GetAccTime) DeltaSeconds)))
    (:then_1
      ;[1 1 1] Go에 True, fals 따른 값 세팅
      (if (Variables|Default|GetGo)
        ;[1 1 1] Then 1로 Cube가 올라가게  세팅
        (Transformation|SetActorLocation (+ (Transformation|GetActorLocation) (* (* (Math|Vector|Normalize (Variables|Default|GetDir)) (Variables|Default|GetSpeed)) DeltaSeconds)) false false)
        (else
          ;[1 1 1] 내려가기
          (Transformation|SetActorLocation (+ (Transformation|GetActorLocation) (* (* (Math|Vector|Normalize (* (Variables|Default|GetDir) -1.0)) (Variables|Default|GetSpeed)) DeltaSeconds)) false false))))
    (:then_2
      ;[1 1 1] Then 2로 AccTime이 3보다크면 0으로 초기화해줌
      (if (> (Variables|Default|GetAccTime) 5.0)
        (if (Variables|Default|GetGo)
          (Variables|Default|SetGo false)
          (else
            (Variables|Default|SetGo true)))
        (Variables|Default|SetAccTime 0.0)))))

(fn ConstructionScript)