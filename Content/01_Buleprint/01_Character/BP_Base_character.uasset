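; BP_Base_character is a base player character providing walk, look and jump controls through Enhanced Input.
; On BeginPlay it adds the IM_Context mapping context to its player controller's local input subsystem.
; Forward and right input move along control-rotation yaw only, so camera pitch does not affect direction.
; Mouse input drives controller yaw and pitch, and the jump action calls Jump when started.
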(event Input|EnhancedActionEvents|EnhancedInputActionIA_Jump
  (params (ActionValue :type Boolean) (ElapsedSeconds :type Float%20%28double-precision%29) (TriggeredSeconds :type Float%20%28double-precision%29) (InputAction :type Input%20Action%20Object%20Reference :default "/Game/01_Buleprint/00_Global/Input/IA_Jump.IA_Jump"))
  (:Started
    (Character|Jump)))

(event Input|EnhancedActionEvents|EnhancedInputActionIA_MoveForward
  (params (ActionValue :type Float%20%28double-precision%29) (ElapsedSeconds :type Float%20%28double-precision%29) (TriggeredSeconds :type Float%20%28double-precision%29) (InputAction :type Input%20Action%20Object%20Reference :default "/Game/01_Buleprint/00_Global/Input/IA_MoveForward.IA_MoveForward"))
  (:Triggered
    (Pawn|Input|AddMovementInput (Math|Vector|GetForwardVector (Math|Rotator|MakeRotator 0.0 0.0 (.yaw (Pawn|GetControlRotation :!class /Script/Engine.Pawn)))) ActionValue false)))

(event Input|EnhancedActionEvents|EnhancedInputActionIA_MoveRight
  (params (ActionValue :type Float%20%28double-precision%29) (ElapsedSeconds :type Float%20%28double-precision%29) (TriggeredSeconds :type Float%20%28double-precision%29) (InputAction :type Input%20Action%20Object%20Reference :default "/Game/01_Buleprint/00_Global/Input/IA_MoveRight.IA_MoveRight"))
  (:Triggered
    (Pawn|Input|AddMovementInput (Math|Vector|GetRightVector (Math|Rotator|MakeRotator 0.0 0.0 (.yaw (Pawn|GetControlRotation :!class /Script/Engine.Pawn)))) ActionValue false)))

(event Input|EnhancedActionEvents|EnhancedInputActionIA_MouseXY
  (params (ActionValue :type Vector%202D%20Structure) (ElapsedSeconds :type Float%20%28double-precision%29) (TriggeredSeconds :type Float%20%28double-precision%29) (InputAction :type Input%20Action%20Object%20Reference :default "/Game/01_Buleprint/00_Global/Input/IA_MouseXY.IA_MouseXY"))
  (:Triggered
    (Pawn|Input|AddControllerYawInput (.x ActionValue))
    (Pawn|Input|AddControllerPitchInput (.y ActionValue))))

(event EventBeginPlay
  (bind _as플레이어_컨트롤러 (Utilities|Casting|CastToPlayerController (Pawn|GetController)))
  (Utilities|IsValid _as플레이어_컨트롤러
    (:Is%20Valid
      (Input|AddMappingContext (PlayerController|LocalPlayerSubsystems|GetEnhancedInputLocalPlayerSubsystem _as플레이어_컨트롤러) "/Game/01_Buleprint/00_Global/Input/IM_Context.IM_Context" 0 "(bIgnoreAllPressedKeysUntilRelease=True,bForceImmediately=False,bNotifyUserSettings=False)"))))

(event Collision|EventActorBeginOverlap
  (params (OtherActor :type Actor%20Object%20Reference)))

(event EventTick
  (params (DeltaSeconds :type Float%20%28single-precision%29)))

(fn ConstructionScript)